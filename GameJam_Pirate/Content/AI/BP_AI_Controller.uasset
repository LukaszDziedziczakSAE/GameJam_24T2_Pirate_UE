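; AI controller for enemies that runs the BT_Enemy behavior tree on BeginPlay.
; An AIPerception update whose actor is the first player character sets the HasSeenPlayer blackboard key to true and prints a debug message.
; The handler does not check whether the player was sensed or lost, and nothing in this controller clears the key.
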(event `self.ReceiveBeginPlay`
  (`self.RunBehaviorTree` "/Game/AI/BT_Enemy.BT_Enemy"))

(event `self.AIPerception.OnTargetPerceptionUpdated`
  (params (Actor :type "Actor Object Reference") (Stimulus :type "AIStimulus Structure"))
  (bind _returnvalue (`GameplayStatics.GetPlayerCharacter` 0))
  (if (== _returnvalue Actor)
    (`BlackboardComponent.SetValueAsBool` (`AIBlueprintHelperLibrary.GetBlackboard` null) "HasSeenPlayer" true)
    (`KismetSystemLibrary.PrintString` (`KismetStringLibrary.Concat_StrStr` (`KismetSystemLibrary.GetDisplayName` self) " saw " (`KismetSystemLibrary.GetDisplayName` _returnvalue)))))

(fn `UserConstructionScript`)