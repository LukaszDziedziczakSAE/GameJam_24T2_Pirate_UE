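; BP_TresureCollectingComponent is a component that tracks treasure collection progress.
; On BeginPlay it counts every BP_TreasureChest actor in the level to set the total to collect, and the CollectedTresure event increments the collected count.
; AmountInArea searches the chests again and returns how many have a LocationIndex matching the given area.
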(event `self.ReceiveBeginPlay`
  (bind _outactors (`GameplayStatics.GetAllActorsOfClass` "/Game/Blueprints/BP_TreasureChest.BP_TreasureChest_C"))
  (set `self.AmountToCollect` (`KismetArrayLibrary.Array_Length` _outactors)))

(event `Collected Tresure`
  (`/Engine/EditorBlueprintResources/StandardMacros.IncrementInt` (`self.AmountCollected`)))

(fn `Amount in Area`
  (params (`Area Index` :type Integer))
  (returns (Amount :type Integer))
  (locals (Count :type Integer))
  (set `local.Count` 0)
  (bind _outactors (`GameplayStatics.GetAllActorsOfClass` "/Game/Blueprints/BP_TreasureChest.BP_TreasureChest_C"))
  (for _array_element _outactors
    (if (== (`/Game/Blueprints/BP_TreasureChest.Location Index` _array_element) `Area Index`)
      (`/Engine/EditorBlueprintResources/StandardMacros.IncrementInt` (`local.Count`))))
  (return (`local.Count`)))