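; BP_PlayerPirate is the player-controlled pirate, handling movement and look through Enhanced Input.
; On BeginPlay it casts its controller to BP_PlayerController and adds the input mapping context to that player's subsystem.
; IA_Look drives controller yaw and pitch, while IA_Move moves along the horizontal components of the camera's forward and right vectors.
; IA_Move also stores the raw axes in ForwardInput and RightInput.
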(event `self.ReceiveBeginPlay`
  (bind _asbp_player_controller (cast `/Game/Blueprints/BP_PlayerController` (`self.GetController`)))
  (bind _returnvalue (pcsubsystem `EnhancedInputLocalPlayerSubsystem` _asbp_player_controller))
  (`/Engine/EditorBlueprintResources/StandardMacros.IsValid` _returnvalue
    (:`Is Valid`
      (`EnhancedInputSubsystemInterface.AddMappingContext` _returnvalue "/Game/Input/InputMappingContext.InputMappingContext" 0 (struct)))))

(event `EnhancedInput|/Game/Input/IA_Look`
  (params (ActionValue :type "Vector2D Structure") (ElapsedSeconds :type "Float (double-precision)") (TriggeredSeconds :type "Float (double-precision)") (InputAction :type "InputAction Object Reference" :default "/Game/Input/IA_Look.IA_Look"))
  (:`Triggered`
    (`self.AddControllerYawInput` ActionValue_X)
    (`self.AddControllerPitchInput` ActionValue_Y)))

(event `EnhancedInput|/Game/Input/IA_Move`
  (params (ActionValue :type "Vector2D Structure") (ElapsedSeconds :type "Float (double-precision)") (TriggeredSeconds :type "Float (double-precision)") (InputAction :type "InputAction Object Reference" :default "/Game/Input/IA_Move.IA_Move"))
  (bind _returnvalue (`SceneComponent.K2_GetComponentRotation` (`self.Camera`)))
  (bind (_returnvalue_x _returnvalue_y) (`KismetMathLibrary.BreakVector` (`KismetMathLibrary.GetForwardVector` _returnvalue)))
  (bind (_returnvalue_x_2 _returnvalue_y_2) (`KismetMathLibrary.BreakVector` (`KismetMathLibrary.GetRightVector` _returnvalue)))
  (:`Triggered`
    (`self.AddMovementInput` (`KismetMathLibrary.MakeVector` _returnvalue_x _returnvalue_y) ActionValue_Y)
    (`self.AddMovementInput` (`KismetMathLibrary.MakeVector` _returnvalue_x_2 _returnvalue_y_2) ActionValue_X)
    (set `self.ForwardInput` ActionValue_Y)
    (set `self.RightInput` ActionValue_X)))

(fn `UserConstructionScript`)