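; BP_TravelArea is a travel point that opens the map view and serves as a destination for the player pirate.
; When the player character overlaps its Box, the player controller switches to the map camera.
; TravelTo prints the area's LocationIndex, teleports the cached pirate to SpawnSpot's position and rotation, then switches the controller back to the game camera.
; Nothing in this Blueprint calls TravelTo.
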(event `self.ReceiveBeginPlay`
  (bind _asbp_player_pirate (cast `/Game/Blueprints/Player/BP_PlayerPirate` (`GameplayStatics.GetPlayerCharacter` 0)))
  (set `self.Player Pirate` _asbp_player_pirate))

(event `self.Box.OnComponentBeginOverlap`
  (params (OverlappedComponent :type "PrimitiveComponent Object Reference") (OtherActor :type "Actor Object Reference") (OtherComp :type "PrimitiveComponent Object Reference") (OtherBodyIndex :type Integer) (bFromSweep :type Boolean) (SweepResult :type "HitResult Structure (by ref)"))
  (bind _returnvalue (`GameplayStatics.GetPlayerCharacter` 0))
  (if (== OtherActor _returnvalue)
    (bind _asbp_player_controller (cast `/Game/Blueprints/BP_PlayerController` (`Pawn.GetController` _returnvalue)))
    (`/Game/Blueprints/BP_PlayerController.Switch to Map Camera` _asbp_player_controller)))

(fn `Travel To`
  (bind _spawnspot (`self.SpawnSpot`))
  (`KismetSystemLibrary.PrintString` (`KismetStringLibrary.Concat_StrStr` "Traveling to " (`KismetStringLibrary.Conv_IntToString` (`self.Location Index`))))
  (`self.K2_SetActorLocationAndRotation` (`self.Player Pirate`) (`SceneComponent.K2_GetComponentLocation` _spawnspot) (`SceneComponent.K2_GetComponentRotation` _spawnspot) true true)
  (bind _asbp_player_controller (cast `/Game/Blueprints/BP_PlayerController` (`Pawn.GetController` (`self.Player Pirate`))))
  (`/Game/Blueprints/BP_PlayerController.Swith to Game Camera` _asbp_player_controller))

(fn `UserConstructionScript`)