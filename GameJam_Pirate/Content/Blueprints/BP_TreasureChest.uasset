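; Treasure chest pickup that the player pirate collects by walking into its overlap sphere.
; The first overlap by player character 0 notifies the TresureCollectingComponent on BP_PlayerPirate, sets a Collected flag so it only counts once, and opens the lid.
; A timeline drives the lid's relative rotation to swing it open.
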(event `self.ReceiveBeginPlay`)

(event `OpenLid`
  (bind (_direction _lidrotation) (`Timeline|LidTransition`)
    (:`Update`
      (`SceneComponent.K2_SetRelativeRotation` (`self.Lid`) (`KismetMathLibrary.RLerp` (struct) (struct :`Roll` -110.0) _lidrotation) false false))))

(event `self.Sphere.OnComponentBeginOverlap`
  (params (OverlappedComponent :type "PrimitiveComponent Object Reference") (OtherActor :type "Actor Object Reference") (OtherComp :type "PrimitiveComponent Object Reference") (OtherBodyIndex :type Integer) (bFromSweep :type Boolean) (SweepResult :type "HitResult Structure (by ref)"))
  (bind _returnvalue (`GameplayStatics.GetPlayerCharacter` 0))
  (if (`self.Collected`)
    _
    (elif (== OtherActor _returnvalue)
      (bind _asbp_player_pirate (cast `/Game/Blueprints/Player/BP_PlayerPirate` _returnvalue))
      (`/Game/Blueprints/BP_TresureCollectingComponent.Collected Tresure` (`/Game/Blueprints/Player/BP_PlayerPirate.Tresure Collecting Component` _asbp_player_pirate))
      (set `self.Collected` true)
      (`self.OpenLid`))))

(fn `UserConstructionScript`)