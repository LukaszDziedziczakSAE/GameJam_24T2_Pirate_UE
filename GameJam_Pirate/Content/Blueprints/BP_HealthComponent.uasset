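; BP_HealthComponent is a health component that tracks damage and triggers death for its owning player pirate or enemy.
; CurrentHealth starts at MaxHealth on BeginPlay, and TakeDamage subtracts from it, clamped between zero and the maximum.
; When IsAlive fails after damage, the Death event casts the owner to BP_PlayerPirate, then BP_EnemyBase, and calls that class's Death.
; Death has no guard, so further damage at zero health triggers it again.
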(event `self.ReceiveBeginPlay`
  (set `self.CurrentHealth` (`self.MaxHealth`)))

(event `Death`
  (bind _returnvalue (`self.GetOwner`))
  (bind _asbp_player_pirate (cast `/Game/Blueprints/Player/BP_PlayerPirate` _returnvalue)
    (:`then`
      (`/Game/Blueprints/Player/BP_PlayerPirate.Death` _asbp_player_pirate))
    (:`CastFailed`
      (bind _asbp_enemy_base (cast `/Game/Enemy/BP_EnemyBase` _returnvalue))
      (`/Game/Enemy/BP_EnemyBase.Death` _asbp_enemy_base))))

(fn `IsAlive`
  (returns (`Is Alive?` :type Boolean))
  (return (> (`self.CurrentHealth`) 0.0)))

(fn `TakeDamage`
  (params (`Damage Amount` :type "Float (double-precision)"))
  (set `self.CurrentHealth` (`KismetMathLibrary.FClamp` (- (`self.CurrentHealth`) `Damage Amount`) 0.0 (`self.MaxHealth`)))
  (if (not (`self.IsAlive`))
    (`self.Death`)))