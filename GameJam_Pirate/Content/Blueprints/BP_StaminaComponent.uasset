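; Stamina component that tracks a current stamina pool, starting at the maximum on BeginPlay.
; Tick regenerates stamina at a per-second rate whenever it is below the maximum, with no active gate or delay after use.
; UseStamina subtracts a clamped amount, while HasStamina and CanAfford report availability.
; CanAfford uses a strict comparison, so spending exactly the remaining stamina is reported as unaffordable.
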(event `self.ReceiveBeginPlay`
  ;[1 1 1] Set Stamina to Maximum Value
  (set `self.CurrentStamina` (`self.MaxStamina`)))

(event `self.ReceiveTick`
  (params (DeltaSeconds :type "Float (single-precision)"))
  ;[1 1 1] Restoration Tick
  (if (< (`self.CurrentStamina`) (`self.MaxStamina`))
    (set `self.CurrentStamina` (`KismetMathLibrary.FClamp` (+ (`self.CurrentStamina`) (* DeltaSeconds (`self.Regeneration Rate`))) 0.0 (`self.MaxStamina`)))))

(fn `Can Afford`
  (params (Amount :type "Float (double-precision)"))
  (returns (`Can Aford` :type Boolean))
  (return (> (- (`self.CurrentStamina`) Amount) 0.0)))

(fn `Has Stamina`
  (returns (`Has Stamina?` :type Boolean))
  (return (> (`self.CurrentStamina`) 0.0)))

(fn `Use Stamina`
  (params (Amount :type "Float (double-precision)"))
  (set `self.CurrentStamina` (`KismetMathLibrary.FClamp` (- (`self.CurrentStamina`) Amount) 0.0 (`self.MaxStamina`))))