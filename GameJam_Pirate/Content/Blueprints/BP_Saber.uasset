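; BP_Saber is a pirate sword weapon that deals melee damage on mesh overlap while it is in use.
; It ignores its owner and actors already hit, then damages the HealthComponent of enemies or the player pirate and spawns an effect at the sweep location.
; WeaponFinished clears the hit list and switches the weapon off, so each target takes damage only once per use.
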(event `self.SM_Pirate_Sword.OnComponentBeginOverlap`
  (params (OverlappedComponent :type "PrimitiveComponent Object Reference") (OtherActor :type "Actor Object Reference") (OtherComp :type "PrimitiveComponent Object Reference") (OtherBodyIndex :type Integer) (bFromSweep :type Boolean) (SweepResult :type "HitResult Structure (by ref)"))
  (if (and (`self.WeaponInUse`) (not (`KismetArrayLibrary.Array_Contains` (`self.DamagedActors`) OtherActor)) (not (== OtherActor (`self.GetOwner`))))
    (`/Engine/EditorBlueprintResources/StandardMacros.IsValid` OtherActor
      (:`Is Valid`
        (`|ExecutionSequence`
          (:`then_0`
            (`KismetSystemLibrary.PrintString` (`KismetStringLibrary.Concat_StrStr` (`KismetSystemLibrary.GetDisplayName` (`self.GetOwner`)) " hit " (`KismetSystemLibrary.GetDisplayName` OtherActor)))
            (bind _asbp_enemy_base (cast `/Game/Enemy/BP_EnemyBase` OtherActor))
            (`KismetArrayLibrary.Array_Add` (`self.DamagedActors`) OtherActor)
            (`/Game/Blueprints/BP_HealthComponent.Take Damage` (`/Game/Enemy/BP_EnemyBase.Health Component` _asbp_enemy_base) (`self.Damage`)))
          (:`then_2`
            (bind _asbp_player_pirate (cast `/Game/Blueprints/Player/BP_PlayerPirate` OtherActor))
            (`KismetArrayLibrary.Array_Add` (`self.DamagedActors`) OtherActor)
            (`/Game/Blueprints/BP_HealthComponent.Take Damage` (`/Game/Blueprints/Player/BP_PlayerPirate.Health Component` _asbp_player_pirate) (`self.Damage`))))
        (`NiagaraFunctionLibrary.SpawnSystemAtLocation` null (`.Location` (`GameplayStatics.BreakHitResult` SweepResult)))))))

(event `Weapon Finished`
  (`KismetArrayLibrary.Array_Clear` (`self.DamagedActors`))
  (set `self.WeaponInUse` false))

(fn `UserConstructionScript`)