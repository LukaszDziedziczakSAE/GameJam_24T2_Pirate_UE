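; BP_PlayerController is the player controller that switches the pirate player between gameplay and map views.
; On BeginPlay it caches the possessed BP_PlayerPirate and the BP_HUD.
; Switching to the map blends the view target to the pirate's TravelSystem map camera, shows the map UI and zeroes the pirate's input.
; Switching back blends the view to the pirate and restores the game UI.
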(event `self.ReceiveBeginPlay`
  (bind _asbp_player_pirate (cast `/Game/Blueprints/Player/BP_PlayerPirate` (`GameplayStatics.GetPlayerPawn` 0)))
  (set `self.Player Pirate` _asbp_player_pirate)
  (bind _asbp_hud (cast `/Game/UI/BP_HUD` (`self.GetHUD`)))
  (set `self.HUD` _asbp_hud))

(event `Switch to Map Camera`
  (bind _player_pirate (`self.Player Pirate`)
    (:`then`
      (`self.SetViewTargetWithBlend` (`/Game/Blueprints/BP_TravelSystem.Map Camera` (`/Game/Blueprints/Player/BP_PlayerPirate.Travel System` _player_pirate)) 0.5)
      (bind _hud (`self.HUD`)
        (:`then`
          (`/Game/UI/BP_HUD.Switch to Map UI` _hud)
          (bind _player_pirate_2 (`self.Player Pirate`)
            (:`then`
              (`/Game/Blueprints/Player/BP_PlayerPirate.Zero Input` _player_pirate_2))
            (:`else`)))
        (:`else`)))
    (:`else`)))

(event `Swith to Game Camera`
  (`self.SetViewTargetWithBlend` (`self.Player Pirate`) 0.5)
  (bind _hud (`self.HUD`)
    (:`then`
      (`/Game/UI/BP_HUD.Switch to Game UI` _hud))
    (:`else`)))

(fn `UserConstructionScript`)